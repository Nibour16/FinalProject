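; Base character Blueprint providing health, death, ground movement speed by state, and martial-arts combo combat.
; Combo montages fire DamageNotify, triggering a socket-based box trace that applies the Attack stat through a DoOnce, limiting damage to one hit per trace.
; Actors of FriendClass are gathered at BeginPlay and ignored by traces unless friendly fire is enabled.
; Damage either destroys the character at zero HP or plays an optional movement-locking hurt montage.
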(event Custom|SetupFriendCharacters
  (bind _friendclass (Variables|Character|Combat|Friend|GetFriendClass))
  ;[0.15 0.15 0.15 0.5] Setup friend characters if Friend Class is set. Character cannot hurt their friends
  (if (Utilities|IsValidClass _friendclass)
    (bind _outactors (Actor|GetAllActorsOfClass _friendclass))
    (for _array_element _outactors
      (if (!= _array_element self)
        (Utilities|Array|AddUnique (Variables|Character|Combat|Friend|GetFriendCharacters) _array_element)))))

(event EventBeginPlay
  ;[0.15 0.15 0.15 0.5] Initialize character movement on ground
  (Character|Movement|SetGroundMovementSpeed)
  (CallFunction|SetupFriendCharacters))

(event Game|Damage|EventAnyDamage
  (params (Damage :type Float%20%28single-precision%29) (DamageType :type Damage%20Type%20Object%20Reference) (InstigatedBy :type Controller%20Object%20Reference) (DamageCauser :type Actor%20Object%20Reference))
  (bind _hurtanimation (Variables|Character|Combat|Animation|Experimental|GetHurtAnimation))
  (bind _charactermovement (Variables|Character|GetCharacterMovement))
  ;[0.15 0.15 0.15 0.5] Character receive damage
  (bind _output_get (Variables|Character|Stat|SetCurrentHP (- (Variables|Character|Stat|GetCurrentHP) Damage)))
  ;[0.15 0.15 0.15 0.5] Call On Dead function if HP runs less or equal to zero, otherwise play hurt animation if the animation is available
  (if (<= _output_get 0.0)
    (Character|OnDead)
    (else
      ;;[1 1 1 1 10] Play hurt Animation (Experimental)
      (Utilities|IsValid _hurtanimation
        (:Is%20Valid
          (Pawn|Components|CharacterMovement|DisableMovement _charactermovement)
          (Animation|Montage|PlayMontage (Variables|Character|GetMesh) _hurtanimation 1.0 0.0 "None" false
            (:OnCompleted
              _)
            (:OnInterrupted
              _))
          (Pawn|Components|CharacterMovement|SetMovementMode _charactermovement "MOVE_Walking" 0))))))

(event Custom|AttackCombo_MartialArts
  (params (GoNextComboWhenFinishAnim :type Boolean))
  ;[0.15 0.15 0.15 0.5] Attack Combo Event support for Maritial Arts Animations only (No weapon)
  (bind _keys (Utilities|Map|Keys (Variables|Character|Combat|Animation|GetAttackComboAnim)))
  (bind (_notifyname _currentcomboanim) (Utilities|PlayAnimationCombo _keys "finishCombo" (Variables|Character|Combat|Animation|GetFinishComboAnimationDelay) GoNextComboWhenFinishAnim 1.0 0.0 "None" true)
    (:On%20Notify%20Begin
      (if (== _notifyname "DamageNotify")
        (if (Variables|Character|Combat|Friend|GetCanAttackFriends)
          (CallFunction|DamageCharacter (.Value (Utilities|Map|Find (Variables|Character|Combat|Animation|GetAttackComboAnim) _currentcomboanim)) "None" 0 5e+01)
          (else
            (CallFunction|DamageCharacter (.Value (Utilities|Map|Find (Variables|Character|Combat|Animation|GetAttackComboAnim) _currentcomboanim)) "None" (Variables|Character|Combat|Friend|GetFriendCharacters) 5e+01)))))))

(event Custom|DamageCharacter
  (params (DamageStartSocket :type Name :default "RightHandSocket") (DamageEndSocket :type Name) (FriendCharacters :type Array%20of%20BP%20Base%20Character%20Object%20References) (HitBoxForwardDistance :type Float%20%28single-precision%29))
  (bind _mesh (Variables|Character|GetMesh))
  (bind _returnvalue (Transformation|GetSocketLocation _mesh DamageStartSocket))
  ;[0.15 0.15 0.15 0.5] Damage Character Event - Make sure to convert the weapon to skeletal mesh and define a specific socket for damage origin point if the character does have it
  (bind _outhits (Class|KismetSystemLibrary|BoxTraceMulti _returnvalue (CallFunction|EndLocationOfInteraction _returnvalue (Utility|TracingEndPositionbySocket DamageEndSocket) HitBoxForwardDistance) (Variables|Character|Combat|GetHitBoxHalfSize) "0, 0, 0" "TraceTypeQuery1" false FriendCharacters "None" true))
  (Utilities|FlowControl|Sequence
    (:then_0
      (goto _label Reset))
    (:then_1
      (for _array_element _outhits
        (Utilities|FlowControl|DoOnce false :!label _label
          (:Completed
            (bind _asbp_base_character (Utilities|Casting|CastToBP_BaseCharacter (.HitActor (Collision|BreakHitResult _array_element))))
            (Game|Damage|ApplyDamage _asbp_base_character (.attack (Variables|Character|Stat|GetCharacterStat)) 0 0)))))))

(fn ConstructionScript
  (bind _mesh (Variables|Character|GetMesh))
  (Utilities|FlowControl|Sequence
    (:then_0
      ;[0.15 0.15 0.15 0.5] Set Mesh relative location to bottom of the Capsule Component and rotation z to -90 degrees when Relative To Capsule is enabled
      (if (Variables|Mesh|GetRelativeToCapsule)
        (Transformation|SetRelativeLocation _mesh (Math|Vector|MakeVector 0.0 0.0 (Utilities|Opposite(Float) (Variables|/Script/Engine.CapsuleComponent|GetCapsuleHalfHeight (Variables|Collision|GetCapsuleComponent)))) false false)
        (Transformation|SetRelativeRotation _mesh "0.000000,-90.000000,0.000000" false false)))
    (:then_1
      ;[0.15 0.15 0.15 0.5] Initialize character's current HP
      (if (Variables|Character|GetStartWithFullHealth)
        (Variables|Character|Stat|SetCurrentHP (.maxhp (Variables|Character|Stat|GetCharacterStat)))
        (else
          (Variables|Character|Stat|SetCurrentHP (Math|Float|Clamp(Float) (Variables|Character|Stat|GetCurrentHP) 0.1 (.maxhp (Variables|Character|Stat|GetCharacterStat)))))))))

(fn OnDead
  (Actor|DestroyActor))

(fn SetGroundMovementState
  (params (NewState :type E_CharacterMovementState%20Enum :default "NewEnumerator0"))
  (Variables|Character|Movement|SetCurrentMovementState NewState)
  (Character|Movement|SetGroundMovementSpeed))

(fn SetGroundMovementSpeed
  (if (Utilities|Enum|Equal(Enum) (Variables|Character|Movement|GetCurrentMovementState) "NewEnumerator0")
    ;[0.15 0.15 0.15 0.5] If current state is standing state will set the move speed to zero
    (Variables|/Script/Engine.CharacterMovementComponent|SetMaxWalkSpeed (Variables|Character|GetCharacterMovement) 0.0)
    (else
      ;[0.15 0.15 0.15 0.5] Set Move speed depending on current state
      (Variables|/Script/Engine.CharacterMovementComponent|SetMaxWalkSpeed (Variables|Character|GetCharacterMovement) (.Value (Utilities|Map|Find (Variables|Character|Movement|Advanced|GetGroundMovementStates) (Variables|Character|Movement|GetCurrentMovementState)))))))

(fn TracingEndPositionbySocket
  (params (EndSocket :type Name))
  (if (Transformation|DoesSocketExist (Variables|Character|GetMesh) EndSocket)
    (return (Transformation|GetSocketLocation (Variables|Character|GetMesh) EndSocket))
    (else
      (return (Transformation|GetActorForwardVector)))))