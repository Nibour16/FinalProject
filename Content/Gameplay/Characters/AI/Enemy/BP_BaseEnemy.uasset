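; Base enemy character Blueprint that links AI sight perception to its controller and manages an overhead health bar.
; Perception updates are filtered to the sight sense, then the target and stimulus go to the AI controller through AssignBlackboardTargetMessage.
; On BeginPlay it sets itself as owner of the WBP_HPBar widget.
; Each tick it turns the bar toward the player camera and can optionally hide it at full health.
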(event OnTargetPerceptionUpdated(AIPerception)
  (params (Actor :type Actor%20Object%20Reference) (Stimulus :type AI%20Stimulus%20Structure))
  ;[0.15 0.15 0.15 0.5] Update Sensing
  (bind _returnvalue (Class|AIPerceptionSystem|GetSenseClassforStimulus Stimulus))
  (Utilities|FlowControl|Sequence
    (:then_0
      (Utilities|CheckDetectedSense _returnvalue "/Script/AIModule.AISense_Sight"
        (:then
          (Class|BIEnemyController|AssignBlackboardTarget(Message) (AI|GetAIController self) Actor Stimulus))))))

(event EventBeginPlay
  ;[0.15 0.15 0.15 0.5] Call Parent function first
  (Utilities|FlowControl|Sequence
    (:then_0
      (|CallParentFunction))
    (:then_1
      ;[0.15 0.15 0.15 0.5] Setup HPBar owner(self)
      (bind _aswbp_hpbar (Utilities|Casting|CastToWBP_HPBar (UserInterface|GetUserWidgetObject (Variables|Default|GetHPBar))))
      (Variables|/Game/Gameplay/Widgets/WBP_HPBar.WBP_HPBar_C|SetOwnerCharacter _aswbp_hpbar self))))

(event EventTick
  (params (DeltaSeconds :type Float%20%28single-precision%29))
  (bind _hpbar (Variables|Default|GetHPBar))
  (Utilities|FlowControl|Sequence
    (:then_0
      ;[0.15 0.15 0.15 0.5] Hide HPBar If it is full health
      (if (Variables|Enemy|GetHideHPBarWhenFullHealth)
        (Development|SetHiddeninGame (Variables|Default|GetHPBar) (CallFunction|IsFullHealth self) false)))
    (:then_1
      ;[0.15 0.15 0.15 0.5] Allow HPBar to always face the player
      (Transformation|SetWorldRotation _hpbar (CallFunction|FindLookatPlayerCamera (Transformation|GetWorldLocation _hpbar)) false false))))

(fn ConstructionScript
  (|CallParentFunction))