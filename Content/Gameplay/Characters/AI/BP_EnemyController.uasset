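; AI controller for enemies that runs the possessed enemy's behavior tree and tracks the player as its target.
; On possess, it records the enemy's origin and injects its behavior subtrees by gameplay tag.
; Sensing a "Player"-tagged actor sets the blackboard Target.
; Losing it opens a gate and starts a delay; re-sensing closes the gate, otherwise Target clears if the enemy can lose targets.
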(event Custom|TargetNotFound
  ;[0.03689 0.03689 0.03689 0.502] Assign Blackboard target variable as player object
  ;;[0.15 0.15 0.15 0.5] When target is not found or lost
  (if (Variables|/Game/Gameplay/Characters/AI/Enemy/BP_BaseEnemy.BP_BaseEnemy_C|GetCanLoseTarget? (Variables|Default|GetEnemyRef))
    ;;;[1 1 1] If can lose target will set the value to null
    (AI|Components|Blackboard|SetValueasObject (Variables|Default|GetBlackboard) (Utilities|Name|MakeLiteralName "Target") 0)))

(event EventPossess
  (params (PossessedPawn :type Pawn%20Object%20Reference))
  ;[0.03689 0.03689 0.03689 0.502] Initialize Enemy's Origin Position and Behaviour Tree
  (bind _asbp_base_enemy (Utilities|Casting|CastToBP_BaseEnemy PossessedPawn))
  (Variables|Default|SetEnemyRef _asbp_base_enemy)
  (Utilities|FlowControl|Sequence
    (:then_0
      (Variables|/Game/Gameplay/Characters/AI/Enemy/BP_BaseEnemy.BP_BaseEnemy_C|SetOriginPos (Variables|Default|GetEnemyRef) (Transformation|GetActorLocation (Variables|Default|GetEnemyRef))))
    (:then_1
      (AI|RunBehaviorTree (Variables|/Game/Gameplay/Characters/AI/Enemy/BP_BaseEnemy.BP_BaseEnemy_C|GetBaseBehaviourTree (Variables|Default|GetEnemyRef))))
    (:then_2
      (bind _asbehavior_tree_component (Utilities|Casting|CastToBehaviorTreeComponent (Variables|Default|GetBrainComponent)))
      (CallFunction|SetBehaviourSubtree (Variables|Default|GetEnemyRef) _asbehavior_tree_component))))

(event EventAssignBlackboardTarget
  (params (TargetActor :type Actor%20Object%20Reference%20%28by%20ref%29) (Stimulus :type AI%20Stimulus%20Structure%20%28by%20ref%29))
  ;[0.03689 0.03689 0.03689 0.502] Assign Blackboard target variable as player object
  ;;[0.15 0.15 0.15 0.5] Check if find a valid target with player tag
  (Utilities|IsValid TargetActor
    (:Is%20Valid
      (if (Utilities|Array|ContainsItem (Variables|/Script/Engine.Actor|GetTags TargetActor) "Player")
        (if (Utilities|Struct|BreakAIStimulus Stimulus)
          (Utilities|FlowControl|Sequence
            (:then_0
              ;;[0.15 0.15 0.15 0.5] When target is found
              (AI|Components|Blackboard|SetValueasObject (Variables|Default|GetBlackboard) (Utilities|Name|MakeLiteralName "Target") TargetActor))
            (:then_1
              (goto _label Close)))
          (else
            ;;[0.15 0.15 0.15 0.5] When target is not found or lost
            (Utilities|FlowControl|Sequence
              (:then_0
                (goto _label Open))
              (:then_1
                (Utilities|FlowControl|Delay 3.0)
                (Utilities|FlowControl|Gate false :!label _label
                  (:Exit
                    (if (Variables|/Game/Gameplay/Characters/AI/Enemy/BP_BaseEnemy.BP_BaseEnemy_C|GetCanLoseTarget? (Variables|Default|GetEnemyRef))
                      ;;;[1 1 1] If can lose target will set the value to null
                      (AI|Components|Blackboard|SetValueasObject (Variables|Default|GetBlackboard) (Utilities|Name|MakeLiteralName "Target") 0))))))))))
    (:Is%20Not%20Valid
      (CallFunction|TargetNotFound))))

(fn ConstructionScript)

(fn SetBehaviourSubtree
  (params (EnemyRef :type BP%20Base%20Enemy%20Object%20Reference) (BehaviourTreeComp :type Behavior%20Tree%20Component%20Object%20Reference))
  (bind (_keypin _valuepin) (Utilities|Map|ForEachLoop(Map) (Variables|/Game/Gameplay/Characters/AI/Enemy/BP_BaseEnemy.BP_BaseEnemy_C|GetBehaviours EnemyRef))
    (:then
      (Class|BehaviorTreeComponent|SetDynamicSubtree BehaviourTreeComp _keypin _valuepin))
    (:CompletedPin
      (return))))